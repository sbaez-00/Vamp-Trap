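; BP_NPC is a talkable NPC that supplies a "Talk to" hover description built from its name.
; Talk starts a dialogue between its speaker component and the player's, binds to the dialogue-ended event, and sends a talk-started event to its StateTree.
; DialogFinished sends the matching talk-finished event to the StateTree.
; Tick derives IsWalking from whether velocity is non-zero, within a tolerance.
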(event `self.ReceiveTick`
  (params (DeltaSeconds :type "Float (single-precision)"))
  (set `self.IsWalking` (not (== (`self.GetVelocity`) (0.0 0.0 0.0) :`ErrorTolerance` 1.0))))

(event `/Game/FirstPerson/Blueprints/BP_Interactable.Talk`
  (params (Player :type "/Game/FirstPerson/Blueprints/BP_FirstPersonCharacter Object Reference"))
  (bind _bpc_speakercomponent (`self.BPC_SpeakerComponent`))
  (`DialogueSpeakerComponent.StartOwnedDialogue` _bpc_speakercomponent (`|MakeArray` _bpc_speakercomponent (`/Game/FirstPerson/Blueprints/BP_FirstPersonCharacter.BPC_SpeakerComponent` Player) :!type "DialogueSpeakerComponent Object Reference") false)
  (add `DialogueController.OnDialogueEnded` (`DialogueSpeakerComponent.DialogueController` _bpc_speakercomponent) (`|CreateDelegate` :!event `DialogFinished`))
  (`StateTreeComponent.SendStateTreeEvent` (`self.StateTree`) (make `StateTreeEvent` (struct :`TagName` "AI.Talk.Started") "test")))

(fn `DialogFinished`
  (`StateTreeComponent.SendStateTreeEvent` (`self.StateTree`) (make `StateTreeEvent` (struct :`TagName` "AI.Talk.Finished"))))

(fn `GetHoverDescription`
  (returns (Description :type String))
  (return (`KismetStringLibrary.Concat_StrStr` "Talk to " (`self.Name`))))

(fn `UserConstructionScript`)